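; BP_CoralBlockSpawner spawns, carries and drops coral blocks, apparently for a stacking game.
; It spawns a random small-scale BlockSet block below itself, passes it the FoulLine, and moves it along with the spawner.
; Release launches the block downward with a set physics velocity, restoring full scale if still shrunk.
; It also exposes block readiness, spawns a BP_HeightChecker from a given center and previous max height, and destroys itself on reset.
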(event EventOnReset
  (Actor|DestroyActor))

(fn ConstructionScript)

(fn CreateBlock
  (bind _returnvalue (Transformation|GetActorTransform))
  (bind _block_set (Variables|Default|GetBlock%20Set))
  (bind _returnvalue_2 (Game|SpawnActorfromClass (Utilities|Array|Get(acopy) _block_set (Math|Random|RandomInteger (Utilities|Array|Length _block_set))) (Math|Transform|MakeTransform (- (.location _returnvalue) "0.000000,0.000000,500.000000") (.rotation _returnvalue) "0.100000,0.100000,0.100000") "Undefined" "MultiplyWithRoot" 0 0))
  (bind _asbp_coral_block (Utilities|Casting|CastToBP_CoralBlock _returnvalue_2))
  (bind _output_get (Variables|Default|SetCurrent%20Block _asbp_coral_block))
  (Variables|/Game/BP_CoralBlock.BP_CoralBlock_C|SetFoul%20Line _output_get (Variables|Default|GetFoul%20Line)))

(fn MoveSpawner
  (params (Action%20Value :type Vector))
  (Transformation|SetActorLocation (- Action%20Value "0.000000,0.000000,100.000000") false false)
  (if (!= (Variables|Default|GetCurrent%20Block) 0)
    (Default|MoveBlock (Variables|Default|GetCurrent%20Block) (Transformation|GetWorldLocation (Variables|Default|GetStaticMesh)))))

(fn ReleaseBlock
  (bind _current_block (Variables|Default|GetCurrent%20Block))
  (bind _staticmesh (Variables|/Game/BP_CoralBlock.BP_CoralBlock_C|GetStaticMesh _current_block))
  (Default|ReleaseBlock (Variables|Default|GetCurrent%20Block))
  (Physics|SetPhysicsLinearVelocity (Variables|/Game/BP_CoralBlock.BP_CoralBlock_C|GetStaticMesh (Variables|Default|GetCurrent%20Block)) "0.000000,0.000000,-350.000000" false "None")
  (if (< (.z (Transformation|GetWorldScale _staticmesh)) 1.0)
    (Transformation|SetWorldScale3D _staticmesh "1.000000,1.000000,1.000000")))

(fn GetCurrentBlockReadiness
  (bind _readiness (Default|GetReadiness (Variables|Default|GetCurrent%20Block)))
  (return _readiness))

(fn SpawnHeightChecker
  (params (Center%20Y :type Float%20%28double-precision%29) (Prev%20Max%20Height :type Float%20%28double-precision%29))
  (bind _staticmesh (Variables|Default|GetStaticMesh))
  (bind _returnvalue (Transformation|GetWorldTransform _staticmesh))
  (bind _returnvalue_2 (Game|SpawnActorfromClass "/Game/BP_HeightChecker.BP_HeightChecker_C" (Math|Transform|MakeTransform (Math|Vector|MakeVector (.x (.location _returnvalue)) Center%20Y Prev%20Max%20Height) (.rotation _returnvalue) (.scale _returnvalue)) "Undefined" "MultiplyWithRoot" 0 0))
  (Variables|Default|SetHeight%20Checker _returnvalue_2))